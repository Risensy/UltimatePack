(fn ShowMouse
  (params (Show%20Mouse%20Cursor :type Boolean) (PC :type Player%20Controller%20Object%20Reference))
  (bind _output_get (Variables|/Script/Engine.PlayerController|SetbShowMouseCursor PC Show%20Mouse%20Cursor))
  (return _output_get))

(fn SetInputMode
  (params (Mode :type E_InputMode%20Enum :default "NewEnumerator0") (PlayerController :type Player%20Controller%20Object%20Reference) (InWidgetToFocus :type Widget%20Object%20Reference) (InMouseLockMode :type EMouseLockMode%20Enum :default "DoNotLock") (bHideCursorDuringCapture :type Boolean) (bFlushInput :type Boolean) (Show%20Mouse%20Cursor :type Boolean))
  (bind _return_value (UI|ShowMouse Show%20Mouse%20Cursor PlayerController))
  (switch Utilities|FlowControl|Switch|SwitchonE_InputMode Mode
    (:NewEnumerator0
      (Input|SetInputModeGameandUI PlayerController InWidgetToFocus InMouseLockMode bHideCursorDuringCapture bFlushInput)
      (return Mode true _return_value))
    (:NewEnumerator1
      (Input|SetInputModeGameOnly PlayerController bFlushInput)
      (return Mode true _return_value))
    (:NewEnumerator2
      (Input|SetInputModeUIOnly PlayerController InWidgetToFocus InMouseLockMode bFlushInput)
      (return Mode true _return_value))))

(fn SetVSync
  (params (bEnable :type Boolean))
  (bind _returnvalue (Settings|GetGameUserSettings))
  (Class|GameUserSettings|SetVSyncEnabled _returnvalue bEnable)
  (return bEnable))

(fn GetUserSettings
  (bind _returnvalue (Settings|GetGameUserSettings))
  (return (Utilities|Struct|MakeS_UserSettings (Class|GameUserSettings|IsVSyncEnabled _returnvalue) (Class|GameUserSettings|GetDesktopResolution _returnvalue) (Class|GameUserSettings|GetFrameRateLimit _returnvalue) (Class|GameUserSettings|GetFullscreenMode _returnvalue) (Class|GameUserSettings|GetSyncInterval _returnvalue) (Class|GameUserSettings|IsHDREnabled _returnvalue) (Class|GameUserSettings|IsDynamicResolutionEnabled _returnvalue) (Class|GameUserSettings|SupportsHDRDisplayOutput _returnvalue))))

(fn SetSpeed
  (params (Character :type Character%20Object%20Reference) (Speed%20Type :type E_CharacterSpeedType%20Enum :default "NewEnumerator0") (Speed :type Float%20%28double-precision%29))
  (switch Utilities|FlowControl|Switch|SwitchonE_CharacterSpeedType Speed%20Type
    (:NewEnumerator0
      (bind _return_value (|Speed Speed (Variables|/Script/Engine.Character|GetCharacterMovement Character) :!label _label)
        (:Out
          (return _return_value))))
    (:NewEnumerator1
      (goto _label Walk))
    (:NewEnumerator2
      (goto _label Swim))
    (:NewEnumerator3
      (goto _label Custom%20Movement))))

(fn PrintBool
  (params (Print%20Type :type E_PrintType%20Enum :default "NewEnumerator0") (Bool :type Boolean) (TextColor :type Linear%20Color%20Structure) (Duration :type Float%20%28single-precision%29) (bPrintToScreen :type Boolean) (bPrintToLog :type Boolean))
  (switch Utilities|FlowControl|Switch|SwitchonE_PrintType Print%20Type
    (:NewEnumerator0
      (Development|PrintText 0 (Utilities|Text|ToText(Boolean) Bool) bPrintToScreen bPrintToLog TextColor Duration))
    (:NewEnumerator1
      (Development|PrintString 0 (Utilities|String|ToString(Boolean) Bool) bPrintToScreen bPrintToLog TextColor Duration)))
  (return true Print%20Type))

(fn CreateWidgetAdvanced
  (params (Class :type User%20Widget%20Class%20Reference) (OwningPlayer :type Player%20Controller%20Object%20Reference) (ZOrder :type Integer) (Show%20Mouse%20Cursor :type Boolean) (Input%20Mode :type E_InputMode%20Enum :default "NewEnumerator0") (InWidgetToFocus :type Widget%20Object%20Reference) (InMouseLockMode :type EMouseLockMode%20Enum :default "DoNotLock") (bHideCursorDuringCapture :type Boolean) (bFlushInput :type Boolean))
  (bind _returnvalue (UserInterface|CreateWidget Class OwningPlayer))
  (UserInterface|Viewport|AddtoViewport _returnvalue ZOrder)
  (UI|ShowMouse Show%20Mouse%20Cursor OwningPlayer)
  (UI|SetInputMode Input%20Mode OwningPlayer InWidgetToFocus InMouseLockMode bHideCursorDuringCapture bFlushInput Show%20Mouse%20Cursor)
  (return true Show%20Mouse%20Cursor))

(fn RemoveWidgetAdvanced
  (params (bShowMouseCursor? :type Boolean) (Target :type Widget%20Object%20Reference) (PC :type Player%20Controller%20Object%20Reference) (Mode :type E_InputMode%20Enum :default "NewEnumerator0") (InMouseLockMode :type EMouseLockMode%20Enum :default "DoNotLock") (bHideCursorDuringCapture :type Boolean) (bFlushInput :type Boolean))
  (Widget|RemovefromParent Target)
  (UI|ShowMouse bShowMouseCursor? PC)
  (bind (_return_mode _return_value _return_show_mouse) (UI|SetInputMode Mode PC 0 InMouseLockMode bHideCursorDuringCapture bFlushInput bShowMouseCursor?))
  (return true _return_mode _return_show_mouse PC))